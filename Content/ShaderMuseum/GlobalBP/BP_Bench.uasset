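; BP_Bench is a bench the player character can sit on and stand up from, toggled through its Sit function.
; Sitting disables movement, teleports the character to the SitPos transform, plays the AM_Sit montage and limits camera yaw around the seated facing.
; Standing restores walking, stops the montage, reopens the yaw limits and re-enables controller-driven yaw.
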(event `SitEvent`
  (bind _returnvalue (`GameplayStatics.GetPlayerCharacter` 0))
  (bind _returnvalue_2 (`GameplayStatics.GetPlayerCharacter` 0))
  (bind (_returnvalue_roll _returnvalue_pitch _returnvalue_yaw) (`KismetMathLibrary.BreakRotator` (`self.K2_GetActorRotation` (`GameplayStatics.GetPlayerCharacter` 0))))
  (bind (_returnvalue_location _returnvalue_rotation) (`KismetMathLibrary.BreakTransform` (`SceneComponent.K2_GetComponentToWorld` (`self.SitPos`))))
  (bind _playercameramanager (`PlayerController.PlayerCameraManager` (`GameplayStatics.GetPlayerController` 0)))
  (`CharacterMovementComponent.DisableMovement` (`Character.CharacterMovement` _returnvalue))
  (`self.K2_SetActorLocationAndRotation` _returnvalue _returnvalue_location _returnvalue_rotation false true)
  (`Controller.SetControlRotation` (`GameplayStatics.GetPlayerController` 0) _returnvalue_rotation)
  (set `Pawn.bUseControllerRotationYaw` false _returnvalue_2)
  (set `PlayerCameraManager.ViewYawMax` (+ _returnvalue_yaw 70.0) _playercameramanager)
  (set `PlayerCameraManager.ViewYawMin` (- _returnvalue_yaw 70.0) _playercameramanager)
  (`|PlayMontage` (`Character.Mesh` _returnvalue_2) "/Game/Core/Characters/Mannequins/Anims/Unarmed/AM_Sit.AM_Sit"))

(event `UnSit`
  (bind _playercameramanager (`PlayerController.PlayerCameraManager` (`GameplayStatics.GetPlayerController` 0)))
  (`CharacterMovementComponent.SetMovementMode` (`Character.CharacterMovement` (`GameplayStatics.GetPlayerCharacter` 0)) "MOVE_Walking" 0)
  (`AnimInstance.Montage_Stop` (`SkeletalMeshComponent.GetAnimInstance` (`Character.Mesh` (`GameplayStatics.GetPlayerCharacter` 0))) 0.1 "/Game/Core/Characters/Mannequins/Anims/Unarmed/AM_Sit.AM_Sit")
  (set `PlayerCameraManager.ViewYawMax` 180.0 _playercameramanager)
  (set `PlayerCameraManager.ViewYawMin` -180.0 _playercameramanager)
  (set `Pawn.bUseControllerRotationYaw` true (`GameplayStatics.GetPlayerCharacter` 0)))

(fn `Sit`
  (if (`self.IsSitting`)
    (`self.UnSit`)
    (set `self.IsSitting` false)
    (else
      (`self.SitEvent`)
      (set `self.IsSitting` true))))

(fn `UserConstructionScript`
  (`parent.UserConstructionScript`))